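; Ground combat unit for either side of a card-based FPS that fights the player or opposing units.
; A self-restarting TargetEnemy loop picks an opponent, with BP_Target overriding for hostiles, then line-traces to choose between shooting projectiles and AI-moving into touch range.
; Flags select stationary, melee-only or self-detonating variants, the latter exploding via BP_Card_Activated.
; Damage and explosive traps feed CheckHealth, which handles death and reports hostile kills to the GameMode.
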(event `self.ReceiveTick`
  (params (DeltaSeconds :type "Float (single-precision)"))
  (`self.AimAtTarget`))

(event `AimAtTarget`
  (bind _targettedenemy (`self.TargettedEnemy`))
  (`/Engine/EditorBlueprintResources/StandardMacros.IsValid` _targettedenemy
    (:`Is Valid`
      (`SceneComponent.K2_SetWorldRotation` (`self.Anchor`) (`KismetMathLibrary.RInterpTo` (`SceneComponent.K2_GetComponentRotation` (`self.Anchor`)) (`KismetMathLibrary.FindLookAtRotation` (`self.K2_GetActorLocation`) (`self.K2_GetActorLocation` _targettedenemy)) (`GameplayStatics.GetWorldDeltaSeconds`) 4.0) false false))))

(event `self.ReceiveBeginPlay`
  (set `self.player` (cast `/Game/FirstPersonBP/Blueprints/FirstPersonCharacter` (`GameplayStatics.GetPlayerPawn` 0) :!pure true))
  (`KismetSystemLibrary.Delay` (`GameplayStatics.GetWorldDeltaSeconds`))
  (`self.TargetEnemy`)
  (set `self.Health` (+ (`self.UpgradeLevel`) (`self.Health`))))

(event `MoveToPlayer`
  (`|AIMoveTo` self (0.0 0.0 0.0) (`self.player`)
    (:`OnSuccess`
      (`/Game/FirstPersonBP/Blueprints/FirstPersonCharacter.TakeDamage` (`self.player`) (`self.Damage_Touch`))
      (`KismetSystemLibrary.Delay` (`self.Delay_Attack_Touch`)))
    (:`OnFail`
      _))
  (`self.MoveToPlayer`))

(event `CheckHealth`
  (if (<= (`self.Health`) 0)
    (if (not (`self.PlayerAlly`))
      (`/Game/Game/GM_LudumDare41.UpdateEnemiesAlive` (cast `/Game/Game/GM_LudumDare41` (`GameplayStatics.GetGameMode`) :!pure true) self))
    (`GameplayStatics.PlaySoundAtLocation` (select `int` (`self.UpgradeLevel`) :`0` "/Game/Sound/Cues/CUE_TankDestroy_0.CUE_TankDestroy_0" :`1` "/Game/Sound/Cues/CUE_TankDestroy_1.CUE_TankDestroy_1" :!type "SoundBase Object Reference") (`self.K2_GetActorLocation`) (struct) 2.5)
    (if (`self.Explodes`)
      (bind _returnvalue (`|SpawnActorFromClass` "/Game/Blueprints/BP_Card_Activated.BP_Card_Activated_C" (`self.GetTransform`) "AlwaysSpawn" "OverrideRootScale" null 0 null))
      (`/Game/Blueprints/BP_Card_Activated.Detonate` _returnvalue))
    (`self.K2_DestroyActor`)))

(event `TakeDamage`
  (params (Damage :type Integer))
  (set `self.Health` (- (`self.Health`) Damage))
  (`self.CheckHealth`))

(event `TargetEnemy`
  (bind _targettedenemy (`self.TargettedEnemy`))
  (bind _damage_touch (`self.Damage_Touch`))
  (bind _targettedenemy_2 (`self.TargettedEnemy`))
  (bind _foundactors (`self.FoundActors`))
  (bind _returnvalue (`KismetMathLibrary.VSize` (- (`self.K2_GetActorLocation`) (`self.K2_GetActorLocation`))))
  (`KismetArrayLibrary.Array_Clear` (`self.FoundActors`))
  (set `self.DistanceCheck` 999999.0)
  (set `self.TargettedEnemy` null)
  (`KismetArrayLibrary.Array_Append` (`self.FoundActors`) (`|MakeArray` (`self.player`) :!type "Actor Object Reference"))
  (if (not (`self.Explodes`))
    (bind _outactors (`GameplayStatics.GetAllActorsOfClass` "/Game/Blueprints/BP_Enemy_Air.BP_Enemy_Air_C"))
    (`KismetArrayLibrary.Array_Append` (`self.FoundActors`) _outactors))
  (bind _outactors_2 (`GameplayStatics.GetAllActorsOfClass` "BP_Enemy_Ground_C"))
  (`KismetArrayLibrary.Array_Append` _foundactors _outactors_2)
  (for _array_element _foundactors
    (cast `/Game/FirstPersonBP/Blueprints/FirstPersonCharacter` _array_element
      (:`then`
        (if (not (`self.PlayerAlly`))
          (if (< _returnvalue (`self.DistanceCheck`)) :!label _label
            (set `self.DistanceCheck` _returnvalue)
            (set `self.TargettedEnemy` _array_element))))
      (:`CastFailed`
        (bind _asbp_enemy_ground (cast `/Game/Blueprints/BP_Enemy_Ground` _array_element)
          (:`then`
            (if (and (!= _array_element self) (!= (`/Game/Blueprints/BP_Enemy_Ground.PlayerAlly` _asbp_enemy_ground) (`self.PlayerAlly`)))
              (goto _label)))
          (:`CastFailed`
            (cast `/Game/Blueprints/BP_Enemy_Air` _array_element)
            (if (and (!= _array_element self) (!= (`/Game/Blueprints/BP_Enemy_Air.PlayerAlly` (cast `/Game/Blueprints/BP_Enemy_Air` _array_element :!pure true)) (`self.PlayerAlly`)))
              (goto _label)))))))
  (if (not (`self.PlayerAlly`))
    (bind _outactors_3 (`GameplayStatics.GetAllActorsOfClass` "/Game/Blueprints/BP_Target.BP_Target_C"))
    (if (> (`KismetArrayLibrary.Array_Length` _outactors_3) 0)
      (set `self.DistanceCheck` 99999.0)
      (for _array_element_2 _outactors_3
        (bind _returnvalue_2 (`KismetMathLibrary.VSize` (- (`self.K2_GetActorLocation` _array_element_2) (`self.K2_GetActorLocation`))))
        (if (< _returnvalue_2 (`self.DistanceCheck`))
          (set `self.DistanceCheck` _returnvalue_2)
          (set `self.TargettedEnemy` _array_element_2)))))
  (`/Engine/EditorBlueprintResources/StandardMacros.IsValid` _targettedenemy
    (:`Is Valid`
      (bind (_outhit _returnvalue_3) (`KismetSystemLibrary.LineTraceSingle` (`self.K2_GetActorLocation`) (`self.K2_GetActorLocation` _targettedenemy) "TraceTypeQuery1"))
      (if _returnvalue_3
        (if (== (`.HitActor` (`GameplayStatics.BreakHitResult` _outhit)) (`self.TargettedEnemy`))
          (if (`self.NoProjectiles`)
            (bind _asbp_enemy_air (cast `/Game/Blueprints/BP_Enemy_Air` (`self.TargettedEnemy`) :!label _label_2)
              (:`then`
                (if (> (.z (`self.K2_GetActorLocation` _asbp_enemy_air)) 150.0)
                  (`|AIMoveTo` self (`KismetMathLibrary.MakeVector` (.x (`self.K2_GetActorLocation` _asbp_enemy_air)) (.y (`self.K2_GetActorLocation` _asbp_enemy_air)) 120.0)
                    (:`OnSuccess`
                      (if (`self.Explodes`) :!label _label_3
                        (bind _returnvalue_4 (`|SpawnActorFromClass` "/Game/Blueprints/BP_Card_Activated.BP_Card_Activated_C" (`self.GetTransform`) "AlwaysSpawn" "OverrideRootScale" null 0 null))
                        (`/Game/Blueprints/BP_Card_Activated.Detonate` _returnvalue_4)
                        (`self.TakeDamage` 200)
                        (else
                          (bind _asbp_enemy_ground_2 (cast `/Game/Blueprints/BP_Enemy_Ground` _targettedenemy_2)
                            (:`then`
                              (`self.TakeDamage` _asbp_enemy_ground_2 _damage_touch))
                            (:`CastFailed`
                              (bind _asfirst_person_character (cast `/Game/FirstPersonBP/Blueprints/FirstPersonCharacter` _targettedenemy_2))
                              (`/Game/FirstPersonBP/Blueprints/FirstPersonCharacter.TakeDamage` _asfirst_person_character _damage_touch)))
                          (`KismetSystemLibrary.Delay` (`self.Delay_Attack_Touch`) :!label _label_4)
                          (`self.TargetEnemy` :!label _label_5))))
                    (:`OnFail`
                      (goto _label_5)))
                  (else
                    (`|AIMoveTo` self (0.0 0.0 0.0) (`self.TargettedEnemy`) :!label _label_6
                      (:`OnSuccess`
                        (goto _label_3))
                      (:`OnFail`
                        (goto _label_5))))))
              (:`CastFailed`
                (goto _label_6)))
            (else
              (`self.ShootAtEnemy`)))
          (elif (`self.Stationary`)
            (goto _label_4)
            (else
              (goto _label_2))))
        (else
          (`KismetSystemLibrary.Delay` (`GameplayStatics.GetWorldDeltaSeconds`) :!label _label_7)
          (`self.TargetEnemy`))))
    (:`Is Not Valid`
      (goto _label_7))))

(event `ShootAtEnemy`
  (bind _returnvalue (`self.K2_GetActorLocation`))
  (`KismetSystemLibrary.Delay` (`KismetMathLibrary.RandomFloatInRange` 0.0 0.2))
  (`|SpawnActorFromClass` "/Game/Blueprints/BP_Projectile.BP_Projectile_C" (`KismetMathLibrary.MakeTransform` _returnvalue (`KismetMathLibrary.FindLookAtRotation` _returnvalue (`self.K2_GetActorLocation` (`self.TargettedEnemy`)))) "Undefined" "OverrideRootScale" null (`self.PlayerAlly`) (`self.Damage_Projectile`) self true (`self.UpgradeLevel`) null)
  (`KismetSystemLibrary.Delay` (`self.Delay_Attack_Projectile`))
  (`self.TargetEnemy`))

(fn `TriggerEffect`
  (params (Effect :type "/Game/Game/ENM_Effect Enum" :default "NewEnumerator0") (Strength :type "Float (double-precision)"))
  (returns (Triggered :type Boolean))
  (switch `/Game/Game/ENM_Effect` Effect
    (:`NewEnumerator0`
      _)
    (:`NewEnumerator1`
      _)
    (:`NewEnumerator2`
      (set `self.Health` (- (`self.Health`) (`KismetMathLibrary.FTrunc` Strength)))
      (`self.CheckHealth`)
      (return true))
    (:`NewEnumerator3`
      _)
    (:`NewEnumerator4`
      _)
    (:`NewEnumerator5`
      _)
    (:`NewEnumerator6`
      _))
  (return false))

(fn `UserConstructionScript`)