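; Flying AI combat unit for the LudumDare41 game that fights for or against the player based on PlayerAlly, starting raised above its spawn point.
; A repeating TargetEnemy loop picks the nearest opposing unit or player, with non-allies preferring BP_Target actors.
; It turns smoothly toward the target, firing projectiles with line of sight, otherwise timeline-lerping to a random, trace-clamped position.
; Damage and explosive traps reduce Health; destruction notifies the game mode.
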(event `self.ReceiveTick`
  (params (DeltaSeconds :type "Float (single-precision)"))
  (`self.AimAtTarget`))

(event `AimAtTarget`
  (bind _targettedenemy (`self.TargettedEnemy`))
  (`/Engine/EditorBlueprintResources/StandardMacros.IsValid` _targettedenemy
    (:`Is Valid`
      (`SceneComponent.K2_SetWorldRotation` (`self.Anchor`) (`KismetMathLibrary.RInterpTo` (`SceneComponent.K2_GetComponentRotation` (`self.Anchor`)) (`KismetMathLibrary.FindLookAtRotation` (`self.K2_GetActorLocation`) (`self.K2_GetActorLocation` _targettedenemy)) (`GameplayStatics.GetWorldDeltaSeconds`) 4.0) false false))))

(event `self.ReceiveBeginPlay`
  (set `self.player` (cast `/Game/FirstPersonBP/Blueprints/FirstPersonCharacter` (`GameplayStatics.GetPlayerPawn` 0) :!pure true))
  (`self.K2_SetActorLocation` (+ (`self.K2_GetActorLocation`) (0.0 0.0 500.0)))
  (`KismetSystemLibrary.Delay` (`GameplayStatics.GetWorldDeltaSeconds`))
  (`self.TargetEnemy`)
  (set `self.Health` (+ (`self.UpgradeLevel`) 1)))

(event `MoveToPlayer`
  (`|AIMoveTo` self (0.0 0.0 0.0) (`self.player`)
    (:`OnSuccess`
      (`/Game/FirstPersonBP/Blueprints/FirstPersonCharacter.TakeDamage` (`self.player`) (`self.Damage_Touch`))
      (`KismetSystemLibrary.Delay` (`self.Delay_Attack_Touch`)))
    (:`OnFail`
      _))
  (`self.MoveToPlayer`))

(event `TakeDamage`
  (params (Damage :type Integer))
  (set `self.Health` (- (`self.Health`) Damage))
  (`self.CheckHealth`))

(event `CheckHealth`
  (if (and (<= (`self.Health`) 0) (not (`self.PlayerAlly`)))
    (`/Game/Game/GM_LudumDare41.UpdateEnemiesAlive` (cast `/Game/Game/GM_LudumDare41` (`GameplayStatics.GetGameMode`) :!pure true) self))
  (`self.K2_DestroyActor`))

(event `TargetEnemy`
  (bind _returnvalue (`self.K2_GetActorLocation`))
  (bind _targettedenemy (`self.TargettedEnemy`))
  (bind _foundactors (`self.FoundActors`))
  (`KismetArrayLibrary.Array_Clear` (`self.FoundActors`))
  (set `self.DistanceCheck` 999999.0)
  (set `self.TargettedEnemy` null)
  (`KismetArrayLibrary.Array_Append` (`self.FoundActors`) (`|MakeArray` (`self.player`) :!type "Actor Object Reference"))
  (bind _outactors (`GameplayStatics.GetAllActorsOfClass` "BP_Enemy_Air_C"))
  (`KismetArrayLibrary.Array_Append` (`self.FoundActors`) _outactors)
  (bind _outactors_2 (`GameplayStatics.GetAllActorsOfClass` "/Game/Blueprints/BP_Enemy_Ground.BP_Enemy_Ground_C"))
  (`KismetArrayLibrary.Array_Append` _foundactors _outactors_2)
  (for _array_element _foundactors
    (cast `/Game/FirstPersonBP/Blueprints/FirstPersonCharacter` _array_element
      (:`then`
        (if (not (`self.PlayerAlly`))
          (bind _returnvalue_2 (`KismetMathLibrary.VSize` (- (`self.K2_GetActorLocation` _array_element) (`self.K2_GetActorLocation`))))
          (if (< _returnvalue_2 (`self.DistanceCheck`)) :!label _label
            (set `self.DistanceCheck` _returnvalue_2)
            (set `self.TargettedEnemy` _array_element))))
      (:`CastFailed`
        (bind _asbp_enemy_ground (cast `/Game/Blueprints/BP_Enemy_Ground` _array_element)
          (:`then`
            (if (and (!= _array_element self) (!= (`/Game/Blueprints/BP_Enemy_Ground.PlayerAlly` _asbp_enemy_ground) (`self.PlayerAlly`)))
              (goto _label)))
          (:`CastFailed`
            (cast `/Game/Blueprints/BP_Enemy_Air` _array_element)
            (if (and (!= _array_element self) (!= (`/Game/Blueprints/BP_Enemy_Air.PlayerAlly` (cast `/Game/Blueprints/BP_Enemy_Air` _array_element :!pure true)) (`self.PlayerAlly`)))
              (goto _label)))))))
  (if (not (`self.PlayerAlly`))
    (bind _outactors_3 (`GameplayStatics.GetAllActorsOfClass` "/Game/Blueprints/BP_Target.BP_Target_C"))
    (if (> (`KismetArrayLibrary.Array_Length` _outactors_3) 0)
      (set `self.DistanceCheck` 99999.0)
      (for _array_element_2 _outactors_3
        (bind _returnvalue_3 (`KismetMathLibrary.VSize` (- (`self.K2_GetActorLocation` _array_element_2) (`self.K2_GetActorLocation`))))
        (if (< _returnvalue_3 (`self.DistanceCheck`))
          (set `self.DistanceCheck` _returnvalue_3)
          (set `self.TargettedEnemy` _array_element_2)))))
  (`/Engine/EditorBlueprintResources/StandardMacros.IsValid` _targettedenemy
    (:`Is Valid`
      (bind _outhit (`KismetSystemLibrary.LineTraceSingle` (`self.K2_GetActorLocation`) (`self.K2_GetActorLocation` _targettedenemy) "TraceTypeQuery1"))
      (if (== (`.HitActor` (`GameplayStatics.BreakHitResult` _outhit)) (`self.TargettedEnemy`))
        (`self.ShootAtEnemy`)
        (else
          (bind _output_get (set `self.SuggestedLocation` (+ _returnvalue (`KismetMathLibrary.MakeVector` (`KismetMathLibrary.RandomFloatInRange` -500.0 500.0) (`KismetMathLibrary.RandomFloatInRange` -500.0 500.0) (`KismetMathLibrary.RandomFloatInRange` -250.0 250.0)))))
          (bind (_outhit_2 _returnvalue_4) (`KismetSystemLibrary.LineTraceSingle` _returnvalue _output_get "TraceTypeQuery1"))
          (bind (_direction _newtrack_0) (`Timeline|Move` :!via `PlayFromStart`)
            (:`Update`
              (`self.K2_SetActorLocation` (`KismetMathLibrary.VLerp` (`self.K2_GetActorLocation`) (select `bool` _returnvalue_4 :`false` (`self.SuggestedLocation`) :`true` (`.ImpactPoint` (`GameplayStatics.BreakHitResult` _outhit_2))) _newtrack_0)))
            (:`Finished`
              (`KismetSystemLibrary.Delay` (`self.Delay_Attack_Touch`))
              (`self.TargetEnemy`))))))
    (:`Is Not Valid`
      (`KismetSystemLibrary.Delay` (`GameplayStatics.GetWorldDeltaSeconds`))
      (`self.TargetEnemy`))))

(event `self.ReceiveDestroyed`
  (`/Game/Game/GM_LudumDare41.UpdateEnemiesAlive` (cast `/Game/Game/GM_LudumDare41` (`GameplayStatics.GetGameMode`) :!pure true) self))

(event `ShootAtEnemy`
  (bind _returnvalue (`self.K2_GetActorLocation`))
  (`|SpawnActorFromClass` "/Game/Blueprints/BP_Projectile.BP_Projectile_C" (`KismetMathLibrary.MakeTransform` _returnvalue (`KismetMathLibrary.FindLookAtRotation` _returnvalue (`self.K2_GetActorLocation` (`self.TargettedEnemy`)))) "Undefined" "OverrideRootScale" null (`self.PlayerAlly`) (`self.Damage_Projectile`) self null)
  (`KismetSystemLibrary.Delay` (`self.Delay_Attack_Projectile`))
  (`self.TargetEnemy`))

(fn `TriggerEffect`
  (params (Effect :type "/Game/Game/ENM_Effect Enum" :default "NewEnumerator0") (Strength :type "Float (double-precision)"))
  (returns (Triggered :type Boolean))
  (switch `/Game/Game/ENM_Effect` Effect
    (:`NewEnumerator0`
      _)
    (:`NewEnumerator1`
      _)
    (:`NewEnumerator2`
      (set `self.Health` (- (`self.Health`) (`KismetMathLibrary.FTrunc` Strength)))
      (`self.CheckHealth`)
      (return true)))
  (return false))

(fn `UserConstructionScript`)