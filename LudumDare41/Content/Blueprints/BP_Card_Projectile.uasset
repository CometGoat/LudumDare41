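; Card projectile that turns into a BP_Card_Activated with the same CardID when it hits a surface, then destroys itself.
; On component hit it prints the impact normal and truncates its components to classify the surface as upward-facing, Y-facing, or everything else.
; That class selects a hand-built rotation aligning the spawned card to the surface, with upward faces also using the projectile's yaw.
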(event `self.CollisionComponent.OnComponentHit`
  (params (HitComponent :type "PrimitiveComponent Object Reference") (OtherActor :type "Actor Object Reference") (OtherComp :type "PrimitiveComponent Object Reference") (NormalImpulse :type "Vector Structure") (Hit :type "HitResult Structure (by ref)"))
  (bind (_bblockinghit _binitialoverlap _time _distance _location _impactpoint _normal _impactnormal) (`GameplayStatics.BreakHitResult` Hit))
  (bind _returnvalue (`KismetMathLibrary.FTrunc` (.y _impactnormal)))
  (`KismetSystemLibrary.PrintString` (`KismetStringLibrary.Conv_VectorToString` _impactnormal))
  (if (== (`KismetMathLibrary.FTrunc` (.z _impactnormal)) 1)
    (set `self.AngleID` 0)
    (elif (or (== _returnvalue 1) (== _returnvalue -1))
      (set `self.AngleID` 1)
      (else
        (if (== (`KismetMathLibrary.FTrunc` (.x _impactnormal)) 1)
          _
          (else
            _))
        (set `self.AngleID` 2))))
  (`|SpawnActorFromClass` "/Game/Blueprints/BP_Card_Activated.BP_Card_Activated_C" (`KismetMathLibrary.MakeTransform` (`self.K2_GetActorLocation`) (select `int` (`self.AngleID`) :`0` (`KismetMathLibrary.ComposeRotators` (`KismetMathLibrary.MakeRotator` (.roll (`KismetMathLibrary.MakeRotFromZ` _impactnormal))) (`KismetMathLibrary.MakeRotator` (.roll (`self.K2_GetActorRotation`)) 0.0 (+ (.yaw (`self.K2_GetActorRotation`)) 180.0))) :`1` (`KismetMathLibrary.ComposeRotators` (`KismetMathLibrary.MakeRotator` 0.0 0.0 (.yaw (`KismetMathLibrary.MakeRotFromY` _impactnormal))) (`KismetMathLibrary.MakeRotator` (select `int` (+ (`KismetMathLibrary.FTrunc` (.y _impactnormal)) 1) :`0` -90.0 :`1` 0.0 :`2` 90.0 :!type "Float (single-precision)") -90.0)) :`2` (`KismetMathLibrary.ComposeRotators` (`KismetMathLibrary.MakeRotator` 0.0 0.0 (.yaw (`KismetMathLibrary.MakeRotFromX` _impactnormal))) (`KismetMathLibrary.MakeRotator` 0.0 (select `int` (+ (`KismetMathLibrary.FTrunc` (.x _impactnormal)) 1) :`0` 90.0 :`1` 0.0 :`2` -90.0 :!type "Float (single-precision)"))))) "AlwaysSpawn" "OverrideRootScale" null (`self.CardID`) null)
  (`self.K2_DestroyActor`))

(fn `UserConstructionScript`
  (`parent.UserConstructionScript`))