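; Projectile fired by ground and air enemies, which can be allied with or hostile to the player, that deals damage on overlap.
; On spawn it plays a tank or moth shot sound picked from shooter type and upgrade level.
; Overlap casts find ground enemies, the player character or air enemies, skipping the shooter and same-side targets.
; A valid target takes damage and the projectile destroys itself; blocking hits have no logic.
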(event `self.ReceiveBeginPlay`
  (`GameplayStatics.SpawnSoundAtLocation` (select `int` (+ (`self.UpgradeLevel`) (select `bool` (`self.GroundEnemy`) :`false` 2)) :`0` "/Game/Sound/SFX/Tank_Shoot_0.Tank_Shoot_0" :`1` "/Game/Sound/SFX/Tank_Shoot_1.Tank_Shoot_1" :`2` "/Game/Sound/SFX/Moth_Shoot_0.Moth_Shoot_0" :`3` "/Game/Sound/SFX/Moth_Shoot_1.Moth_Shoot_1" :!type "SoundBase Object Reference") (`self.K2_GetActorLocation`) (struct) 2.5))

(event `self.CollisionComponent.OnComponentHit`
  (params (HitComponent :type "PrimitiveComponent Object Reference") (OtherActor :type "Actor Object Reference") (OtherComp :type "PrimitiveComponent Object Reference") (NormalImpulse :type "Vector Structure") (Hit :type "HitResult Structure (by ref)")))

(event `self.CollisionComponent.OnComponentBeginOverlap`
  (params (OverlappedComponent :type "PrimitiveComponent Object Reference") (OtherActor :type "Actor Object Reference") (OtherComp :type "PrimitiveComponent Object Reference") (OtherBodyIndex :type Integer) (bFromSweep :type Boolean) (SweepResult :type "HitResult Structure (by ref)"))
  (bind _damage (`self.Damage`))
  (bind _asbp_enemy_ground (cast `/Game/Blueprints/BP_Enemy_Ground` OtherActor)
    (:`then`
      (if (!= _asbp_enemy_ground (`self.ShootingActor`))
        (if (!= (`/Game/Blueprints/BP_Enemy_Ground.PlayerAlly` _asbp_enemy_ground) (`self.PlayerAlly`))
          (`/Game/Blueprints/BP_Enemy_Ground.TakeDamage` _asbp_enemy_ground _damage)
          (`self.K2_DestroyActor` :!label _label))))
    (:`CastFailed`
      (bind _asfirst_person_character (cast `/Game/FirstPersonBP/Blueprints/FirstPersonCharacter` OtherActor)
        (:`then`
          (if (not (`self.PlayerAlly`))
            (`/Game/FirstPersonBP/Blueprints/FirstPersonCharacter.TakeDamage` _asfirst_person_character _damage)
            (goto _label)))
        (:`CastFailed`
          (bind _asbp_enemy_air (cast `/Game/Blueprints/BP_Enemy_Air` OtherActor))
          (if (and (!= _asbp_enemy_air (`self.ShootingActor`)) (!= (`/Game/Blueprints/BP_Enemy_Air.PlayerAlly` _asbp_enemy_air) (`self.PlayerAlly`)))
            (`/Game/Blueprints/BP_Enemy_Air.TakeDamage` _asbp_enemy_air (`self.Damage`))
            (goto _label)))))))

(fn `UserConstructionScript`
  (`parent.UserConstructionScript`))