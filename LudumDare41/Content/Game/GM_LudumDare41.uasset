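; Game mode for a Ludum Dare 41 first-person card-battler that runs the main menu, deck building and a wave-based round loop.
; Each round clears the arena, resets the player and hand, then recursively spawns random weighted enemies at spawn points away from the player.
; Clearing a wave returns to deck building with rising difficulty and enemy counts, until passing round ten triggers player success.
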(event `ResetArena`
  (bind _outactors (`GameplayStatics.GetAllActorsOfClass` "/Game/Blueprints/BP_Enemy_Air.BP_Enemy_Air_C"))
  (for _array_element _outactors
    (`self.K2_DestroyActor` _array_element))
  (bind _outactors_2 (`GameplayStatics.GetAllActorsOfClass` "/Game/Blueprints/BP_Enemy_Ground.BP_Enemy_Ground_C"))
  (for _array_element_2 _outactors_2
    (`self.K2_DestroyActor` _array_element_2))
  (bind _outactors_3 (`GameplayStatics.GetAllActorsOfClass` "/Game/Blueprints/BP_Card_Activated.BP_Card_Activated_C"))
  (for _array_element_3 _outactors_3
    (`self.K2_DestroyActor` _array_element_3))
  (bind _outactors_4 (`GameplayStatics.GetAllActorsOfClass` "/Game/Blueprints/BP_Wall.BP_Wall_C"))
  (for _array_element_4 _outactors_4
    (`self.K2_DestroyActor` _array_element_4)))

(event `BuildDeck`
  (bind _returnvalue (`GameplayStatics.GetPlayerController` 0))
  (`/Engine/EditorBlueprintResources/StandardMacros.DecrementInt` (`self.DeckStartSize`)
    (:`  `
      (bind _returnvalue_2 (`|CreateWidget` "/Game/UI/Widgets/W_CardSelector.W_CardSelector_C" _returnvalue true (`self.DeckStartSize`)))
      (`UserWidget.AddToViewport` _returnvalue_2 0)
      (`WidgetBlueprintLibrary.SetInputMode_UIOnlyEx` _returnvalue _returnvalue_2)
      (set `PlayerController.bShowMouseCursor` true _returnvalue)
      (`/Game/UI/Widgets/W_HUD.UpdateEnemiesLeft` (`self.W_HUD`) true (`KismetMathLibrary.FTrunc` (* (`self.EnemiesPerRound`) (/ (`KismetMathLibrary.Conv_IntToDouble` (`self.Round_Next`)) 2.0)))))))

(event `self.ReceiveBeginPlay`
  (bind _returnvalue (`GameplayStatics.GetPlayerController` 0))
  (bind _returnvalue_2 (`|CreateWidget` "/Game/UI/Widgets/W_MainMenu.W_MainMenu_C"))
  (`UserWidget.AddToViewport` _returnvalue_2 0)
  (`self.DisableInput` (`GameplayStatics.GetPlayerPawn` 0) _returnvalue)
  (`WidgetBlueprintLibrary.SetInputMode_UIOnlyEx` _returnvalue _returnvalue_2)
  (set `PlayerController.bShowMouseCursor` true _returnvalue)
  (`GameplayStatics.PlaySound2D` "/Game/Sound/Music/LDJam41.LDJam41"))

(event `PlayGame`
  (bind _outactors (`GameplayStatics.GetAllActorsOfClass` "/Game/Blueprints/BP_Spawn.BP_Spawn_C"))
  (set `self.Spawns` _outactors)
  (set `self.Player` (cast `/Game/FirstPersonBP/Blueprints/FirstPersonCharacter` (`GameplayStatics.GetPlayerPawn` 0) :!pure true))
  (`KismetSystemLibrary.Delay` (`GameplayStatics.GetWorldDeltaSeconds`))
  (`self.BuildDeck`))

(event `NewRound`
  (bind _player (`self.Player`))
  (bind _player_2 (`self.Player`))
  (bind _returnvalue (`KismetMathLibrary.FTrunc` (* (`self.EnemiesPerRound`) (/ (`KismetMathLibrary.Conv_IntToDouble` (`self.Round_Next`)) 2.0))))
  (`|ExecutionSequence`
    (:`then_0`
      (`/Engine/EditorBlueprintResources/StandardMacros.DoOnce` false
        (:`Completed`
          (`/Game/FirstPersonBP/Blueprints/FirstPersonCharacter.StartGame` (`self.Player`)))))
    (:`then_1`
      (`self.EnableInput` (`GameplayStatics.GetPlayerPawn` 0) (`GameplayStatics.GetPlayerController` 0))
      (set `self.SpawnDelay` (* (`self.SpawnDelay`) 0.94))
      (`self.ResetArena`)
      (`PrimitiveComponent.SetCollisionEnabled` (`Character.CapsuleComponent` (cast `/Game/FirstPersonBP/Blueprints/FirstPersonCharacter` (`GameplayStatics.GetPlayerPawn` 0) :!pure true)) "QueryAndPhysics")
      (`/Game/FirstPersonBP/Blueprints/FirstPersonCharacter.ResetAttributes` _player_2)
      (`self.EnableInput` (`self.Player`) (`GameplayStatics.GetPlayerController` 0))
      (`/Game/FirstPersonBP/Blueprints/FirstPersonCharacter.RefreshDeck` _player)
      (`/Game/FirstPersonBP/Blueprints/FirstPersonCharacter.DrawNewHand` _player)
      (bind _returnvalue_2 (`|CreateWidget` "/Game/UI/Widgets/W_Timer.W_Timer_C"))
      (`UserWidget.AddToViewport` _returnvalue_2 0)
      (`/Game/UI/Widgets/W_HUD.UpdateEnemiesLeft` (`self.W_HUD`) true _returnvalue)
      (`KismetSystemLibrary.Delay` (+ (`/Game/FirstPersonBP/Blueprints/FirstPersonCharacter.DrawDelay` _player) 1.0))
      (set `/Game/FirstPersonBP/Blueprints/FirstPersonCharacter.InBattle` true _player_2)
      (set `self.EnemiesToSpawn` _returnvalue)
      (set `self.ShowEnemiesAlive` false)
      (`KismetArrayLibrary.Array_Clear` (`self.EnemiesLeft`))
      (`self.SpawnEnemies`))))

(event `SpawnEnemies`
  (bind _spawns (`self.Spawns`))
  (bind _enemiestospawn (`self.EnemiesToSpawn`))
  (bind _player (`self.Player`))
  (bind _player_2 (`self.Player`))
  (bind _str_enemy_database_enemies (break `/Game/Game/STR_Enemy_Database` (`self.STR_Enemy_Database`)))
  (bind _newenemydifficulty (`self.NewEnemyDifficulty`))
  (bind _returnvalue (`self.K2_GetActorLocation` (`self.SelectedSpawn`)))
  (bind _cardids (`/Game/FirstPersonBP/Blueprints/FirstPersonCharacter.CardIDs` _player))
  (`KismetSystemLibrary.Delay` (`self.SpawnDelay`))
  (set `self.SelectedSpawn` (`|GetArrayItem` _spawns (`KismetMathLibrary.RandomIntegerInRange` 0 (`KismetArrayLibrary.Array_LastIndex` _spawns))) :!label _label)
  (if (>= (`KismetMathLibrary.VSize` (- (`self.K2_GetActorLocation` (`self.Player`)) (`self.K2_GetActorLocation` (`self.SelectedSpawn`)))) 512.0)
    (bind _output_get (set `self.SuggestedEnemy` (`KismetMathLibrary.RandomIntegerInRange` 0 (`KismetArrayLibrary.Array_LastIndex` _str_enemy_database_enemies)) :!label _label_2))
    (if (== _output_get 2)
      (goto _label_2)
      (else
        (if (== _output_get 3)
          (if (== (`KismetMathLibrary.RandomIntegerInRange` 0 3) 0)
            _
            (else
              (goto _label_2))))
        (bind _output_get_2 (set `self.NewEnemyDifficulty` (`KismetMathLibrary.FTrunc` (`KismetMathLibrary.FClamp` (* (`KismetMathLibrary.RandomFloatInRange` 0.0 0.5) (`self.Difficulty`))))))
        (bind _returnvalue_2 (+ (`KismetMathLibrary.Conv_IntToDouble` _output_get_2) 1.0))
        (bind _returnvalue_3 (`|SpawnActorFromClass` (`|GetArrayItem` _str_enemy_database_enemies (`self.SuggestedEnemy`)) (`KismetMathLibrary.MakeTransform` _returnvalue (`KismetMathLibrary.FindLookAtRotation` _returnvalue (`self.K2_GetActorLocation` (`self.Player`))) (`KismetMathLibrary.MakeVector` _returnvalue_2 _returnvalue_2 _returnvalue_2)) "AdjustIfPossibleButAlwaysSpawn" "OverrideRootScale" null null))
        (bind _returnvalue_4 (`self.K2_GetActorLocation` _returnvalue_3))
        (`GameplayStatics.SpawnEmitterAtLocation` "/Game/StarterContent/Particles/P_Summon.P_Summon" _returnvalue_4 (struct) (1.6 1.6 1.6))
        (`GameplayStatics.PlaySoundAtLocation` "/Game/Sound/Cues/CUE_Summon.CUE_Summon" _returnvalue_4)
        (`KismetArrayLibrary.Array_Add` (`self.EnemiesLeft`) _returnvalue_3)
        (bind _asbp_enemy_ground (cast `/Game/Blueprints/BP_Enemy_Ground` _returnvalue_3)
          (:`then`
            (set `/Game/Blueprints/BP_Enemy_Ground.UpgradeLevel` _newenemydifficulty _asbp_enemy_ground))
          (:`CastFailed`
            (bind _asbp_enemy_air (cast `/Game/Blueprints/BP_Enemy_Air` _returnvalue_3))
            (set `/Game/Blueprints/BP_Enemy_Air.UpgradeLevel` _newenemydifficulty _asbp_enemy_air)))
        (`/Engine/EditorBlueprintResources/StandardMacros.IncrementInt` (`self.EnemiesAlive`)
          (:`  `
            (`/Engine/EditorBlueprintResources/StandardMacros.DecrementInt` _enemiestospawn
              (:`  `
                (`/Game/UI/Widgets/W_HUD.UpdateEnemiesLeft` (`self.W_HUD`) true _enemiestospawn)
                (if (> (`self.EnemiesToSpawn`) 0)
                  (`self.SpawnEnemies`)
                  (else
                    (`/Engine/EditorBlueprintResources/StandardMacros.IncrementInt` (`self.Round_Next`)
                      (:`  `
                        (set `self.ShowEnemiesAlive` true)
                        (`/Game/UI/Widgets/W_HUD.UpdateEnemiesLeft` (`self.W_HUD`) false (`self.EnemiesAlive`))
                        (set `self.Difficulty` (+ (`self.Difficulty`) 0.5))
                        (if (== (`self.EnemiesAlive`) 0) :!label _label_3
                          (`self.DisableInput` _player_2 (`GameplayStatics.GetPlayerController` 0))
                          (set `/Game/FirstPersonBP/Blueprints/FirstPersonCharacter.InBattle` false _player_2)
                          (for (_ _array_index) _cardids
                            (`KismetArrayLibrary.Array_Set` _cardids _array_index -1))
                          (`PanelWidget.ClearChildren` (`/Game/UI/Widgets/W_HUD.Hand` (`/Game/FirstPersonBP/Blueprints/FirstPersonCharacter.W_HUD` _player)))
                          (set `self.DeckStartSize` 2)
                          (if (> (`self.Round_Next`) 10)
                            (`/Game/FirstPersonBP/Blueprints/FirstPersonCharacter.Success` (`self.Player`))
                            (else
                              (`self.BuildDeck`)
                              (`/Game/UI/Widgets/W_HUD.UpdateRoundNumber` (`self.W_HUD`) (`self.Round_Next`)))))))))))))))
    (else
      (goto _label))))

(event `UpdateEnemiesAlive`
  (params (Enemy :type "Actor Object Reference"))
  (bind _returnvalue (`KismetArrayLibrary.Array_RemoveItem` (`self.EnemiesLeft`) Enemy))
  (if _returnvalue
    (`/Engine/EditorBlueprintResources/StandardMacros.DecrementInt` (`self.EnemiesAlive`)
      (:`  `
        (if (`self.ShowEnemiesAlive`)
          (`/Game/UI/Widgets/W_HUD.UpdateEnemiesLeft` (`self.W_HUD`) false (`self.EnemiesAlive`))
          (goto _label_3))))))

(fn `UserConstructionScript`)